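; Player character Blueprint that handles camera look, movement and jumping through Enhanced Input.
; BeginPlay adds the input mapping context to player 0's local subsystem.
; Look input sets yaw through the controller but pitches the capsule itself, whose forward and right vectors also steer movement.
; A camera-lowering crouch step exists but is unconnected and never runs.
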(event Input|EnhancedActionEvents|EnhancedInputActionInputCamera
  (params (ActionValue :type Vector%202D%20Structure) (ElapsedSeconds :type Float%20%28double-precision%29) (TriggeredSeconds :type Float%20%28double-precision%29) (InputAction :type Input%20Action%20Object%20Reference :default "/Game/Inputs/Actions/InputCamera.InputCamera"))
  (bind _cam_rot_speed (Variables|Default|GetCam%20Rot%20Speed))
  ;[1 1 1] Camera Controls
  (:Triggered
    (Transformation|AddLocalRotation (Variables|Collision|GetCapsuleComponent) (Math|Rotator|MakeRotator 0.0 (* (.y ActionValue) _cam_rot_speed) 0.0) false false)
    (Pawn|Input|AddControllerYawInput (* (.x ActionValue) _cam_rot_speed))))

(event Input|EnhancedActionEvents|EnhancedInputActionInputJumpIA
  (params (ActionValue :type Boolean) (ElapsedSeconds :type Float%20%28double-precision%29) (TriggeredSeconds :type Float%20%28double-precision%29) (InputAction :type Input%20Action%20Object%20Reference :default "/Game/Inputs/Actions/InputJumpIA.InputJumpIA"))
  (:Triggered
    (Character|Jump)))

(event Input|EnhancedActionEvents|EnhancedInputActionInputMovement
  (params (ActionValue :type Vector%202D%20Structure) (ElapsedSeconds :type Float%20%28double-precision%29) (TriggeredSeconds :type Float%20%28double-precision%29) (InputAction :type Input%20Action%20Object%20Reference :default "/Game/Inputs/Actions/InputMovement.InputMovement"))
  (bind _move_speed (Variables|Default|GetMove%20Speed))
  (bind _capsulecomponent (Variables|Collision|GetCapsuleComponent))
  ;[1 1 1] Basic 3d Movement
  (:Triggered
    (Pawn|Input|AddMovementInput (Math|Vector|GetForwardVector _capsulecomponent) (* _move_speed (.y ActionValue)) false)
    (Pawn|Input|AddMovementInput (Math|Vector|GetRightVector _capsulecomponent) (* _move_speed (.x ActionValue)) false)))

(event Input|EnhancedActionEvents|EnhancedInputActionInputCrouchIA
  (params (ActionValue :type Boolean) (ElapsedSeconds :type Float%20%28double-precision%29) (TriggeredSeconds :type Float%20%28double-precision%29) (InputAction :type Input%20Action%20Object%20Reference :default "/Game/Inputs/Actions/InputCrouchIA.InputCrouchIA")))

(event EventBeginPlay
  (CallFunction|InitMappingContext))

(fn ConstructionScript)

(fn InitMappingContext
  (Input|AddMappingContext (PlayerController|LocalPlayerSubsystems|GetEnhancedInputLocalPlayerSubsystem (Game|GetPlayerController 0)) "/Game/Inputs/InputMapping.InputMapping" 0 "(bIgnoreAllPressedKeysUntilRelease=True,bForceImmediately=False)"))