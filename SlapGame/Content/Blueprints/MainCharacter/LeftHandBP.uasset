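; LeftHandBP is a main-character hand actor that pushes whatever its CubeColl collider overlaps.
; Right-click press and release events switch CubeColl between query-and-physics collision and no collision, so it only hits while active.
; On begin overlap it sends YouHAveBeenPushedMessage to the other actor with the collider's forward vector as the push direction, printing debug strings along the way.
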(event EventBeginPlay)

(event Collision|EventActorBeginOverlap
  (params (OtherActor :type Actor%20Object%20Reference)))

(event EventTick
  (params (DeltaSeconds :type Float%20%28single-precision%29)))

(event EventRightClickPresed
  (params (Pressed :type Boolean))
  (Collision|SetCollisionEnabled (Variables|Default|GetCubeColl) "QueryAndPhysics")
  (Development|PrintString "HitRight"))

(event EventRightClickUnPressed
  (Collision|SetCollisionEnabled (Variables|Default|GetCubeColl) "NoCollision")
  (Development|PrintString "Hello"))

(fn ConstructionScript)

(event OnComponentBeginOverlap(CubeColl)
  (params (OverlappedComponent :type Primitive%20Component%20Object%20Reference) (OtherActor :type Actor%20Object%20Reference) (OtherComp :type Primitive%20Component%20Object%20Reference) (OtherBodyIndex :type Integer) (bFromSweep :type Boolean) (SweepResult :type Hit%20Result%20Structure%20%28by%20ref%29))
  (bind _cubecoll (Variables|Default|GetCubeColl))
  (bind _returnvalue (Math|Vector|GetForwardVector _cubecoll))
  (Development|PrintString (Utilities|String|ToString(Vector) _returnvalue))
  (Class|PlayerInterface|YouHAveBeenPushed(Message) OtherActor _returnvalue)
  (Development|PrintString (Utilities|GetDisplayName OtherActor)))