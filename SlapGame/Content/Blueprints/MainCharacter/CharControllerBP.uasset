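; CharControllerBP is the main character Blueprint, handling look, movement and left-hand input through Enhanced Input.
; On BeginPlay it adds the input mapping context and caches the LeftHandBP child actor.
; Look input adds controller yaw but pitches the capsule itself, whose forward and right vectors drive movement.
; Hand input start is forwarded to the left hand as a right-click press, and cancel or completion as a release.
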(event Input|EnhancedActionEvents|EnhancedInputActionInputHands
  (params (ActionValue :type Boolean) (ElapsedSeconds :type Float%20%28double-precision%29) (TriggeredSeconds :type Float%20%28double-precision%29) (InputAction :type Input%20Action%20Object%20Reference :default "/Game/Inputs/Actions/InputHands.InputHands"))
  (bind _lhreference (Variables|Default|GetlHReference))
  (:Started
    (Default|RightClickPresed _lhreference ActionValue))
  (:Canceled
    (Class|PlayerInterface|RightClickUnPressed(Message) _lhreference :!label _label))
  (:Completed
    (goto _label)))

(event Input|EnhancedActionEvents|EnhancedInputActionInputMovement
  (params (ActionValue :type Vector%202D%20Structure) (ElapsedSeconds :type Float%20%28double-precision%29) (TriggeredSeconds :type Float%20%28double-precision%29) (InputAction :type Input%20Action%20Object%20Reference :default "/Game/Inputs/Actions/InputMovement.InputMovement"))
  (bind _capsulecomponent (Variables|Collision|GetCapsuleComponent))
  (bind _move_speed (Variables|Default|GetMove%20Speed))
  (:Triggered
    (Pawn|Input|AddMovementInput (Math|Vector|GetForwardVector _capsulecomponent) (* _move_speed (.y ActionValue)) false)
    (Pawn|Input|AddMovementInput (Math|Vector|GetRightVector _capsulecomponent) (* _move_speed (.x ActionValue)) false)))

(event Input|EnhancedActionEvents|EnhancedInputActionInputCamera
  (params (ActionValue :type Vector%202D%20Structure) (ElapsedSeconds :type Float%20%28double-precision%29) (TriggeredSeconds :type Float%20%28double-precision%29) (InputAction :type Input%20Action%20Object%20Reference :default "/Game/Inputs/Actions/InputCamera.InputCamera"))
  (bind _cam_rot_speed (Variables|Default|GetCam%20Rot%20Speed))
  (:Triggered
    (Transformation|AddLocalRotation (Variables|Collision|GetCapsuleComponent) (Math|Rotator|MakeRotator 0.0 (* (.y ActionValue) _cam_rot_speed) 0.0) false false)
    (Pawn|Input|AddControllerYawInput (* (.x ActionValue) _cam_rot_speed))))

(event EventBeginPlay
  (Development|PrintString "IRENE : CharController BeginPlay")
  (CallFunction|InitMappingContext)
  (bind _asleft_hand_bp (Utilities|Casting|CastToLeftHandBP (Variables|/Script/Engine.ChildActorComponent|GetChildActor (Variables|Default|GetLeftHandBP))))
  (Variables|Default|SetlHReference _asleft_hand_bp))

(fn ConstructionScript)

(fn InitMappingContext
  (Input|AddMappingContext (PlayerController|LocalPlayerSubsystems|GetEnhancedInputLocalPlayerSubsystem (Game|GetPlayerController 0)) "/Game/Inputs/InputMapping.InputMapping" 0 "(bIgnoreAllPressedKeysUntilRelease=True,bForceImmediately=False)"))